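; BP_DefaultCell is a cell actor that visualizes its interaction state through its mesh material.
; On BeginPlay it creates a dynamic instance of M_CellMaterial, waits one tick, then passes CellVariationIndex into it as a scalar parameter.
; OnStateChanged sets mutually exclusive scalar flags for hovered, selected, available and unavailable, clearing all of them for any other state.
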(event `self.ReceiveBeginPlay`
  (bind _returnvalue (`PrimitiveComponent.CreateDynamicMaterialInstance` (`self.cellMesh`) 0 "/Game/_Game/Core/Cells/M_CellMaterial.M_CellMaterial" "None"))
  (set `self.MaterialInstance` _returnvalue)
  (`KismetSystemLibrary.DelayUntilNextTick`)
  (`MaterialInstanceDynamic.SetScalarParameterValue` (`self.MaterialInstance`) "CellVariationIndex" (`KismetMathLibrary.Conv_IntToDouble` (`self.cellVariationIndex`))))

(event `self.OnStateChanged`
  (params (newState :type "EChessCellState Enum" :default "Default"))
  (switch `EChessCellState` newState
    (:`Default`
      (`MaterialInstanceDynamic.SetScalarParameterValue` (`self.MaterialInstance`) "IsHovered" 0.0)
      (`MaterialInstanceDynamic.SetScalarParameterValue` (`self.MaterialInstance`) "IsSelected" 0.0)
      (`MaterialInstanceDynamic.SetScalarParameterValue` (`self.MaterialInstance`) "IsAvaible" 0.0)
      (`MaterialInstanceDynamic.SetScalarParameterValue` (`self.MaterialInstance`) "IsUnavaible" 0.0))
    (:`Hovered`
      (`MaterialInstanceDynamic.SetScalarParameterValue` (`self.MaterialInstance`) "IsHovered" 1.0)
      (`MaterialInstanceDynamic.SetScalarParameterValue` (`self.MaterialInstance`) "IsSelected" 0.0)
      (`MaterialInstanceDynamic.SetScalarParameterValue` (`self.MaterialInstance`) "IsAvaible" 0.0)
      (`MaterialInstanceDynamic.SetScalarParameterValue` (`self.MaterialInstance`) "IsUnavaible" 0.0))
    (:`Selected`
      (`MaterialInstanceDynamic.SetScalarParameterValue` (`self.MaterialInstance`) "IsHovered" 0.0)
      (`MaterialInstanceDynamic.SetScalarParameterValue` (`self.MaterialInstance`) "IsSelected" 1.0)
      (`MaterialInstanceDynamic.SetScalarParameterValue` (`self.MaterialInstance`) "IsAvaible" 0.0)
      (`MaterialInstanceDynamic.SetScalarParameterValue` (`self.MaterialInstance`) "IsUnavaible" 0.0))
    (:`Avaible`
      (`MaterialInstanceDynamic.SetScalarParameterValue` (`self.MaterialInstance`) "IsHovered" 0.0)
      (`MaterialInstanceDynamic.SetScalarParameterValue` (`self.MaterialInstance`) "IsSelected" 0.0)
      (`MaterialInstanceDynamic.SetScalarParameterValue` (`self.MaterialInstance`) "IsAvaible" 1.0)
      (`MaterialInstanceDynamic.SetScalarParameterValue` (`self.MaterialInstance`) "IsUnavaible" 0.0))
    (:`Unavaible`
      (`MaterialInstanceDynamic.SetScalarParameterValue` (`self.MaterialInstance`) "IsHovered" 0.0)
      (`MaterialInstanceDynamic.SetScalarParameterValue` (`self.MaterialInstance`) "IsSelected" 0.0)
      (`MaterialInstanceDynamic.SetScalarParameterValue` (`self.MaterialInstance`) "IsAvaible" 0.0)
      (`MaterialInstanceDynamic.SetScalarParameterValue` (`self.MaterialInstance`) "IsUnavaible" 1.0))))

(fn `UserConstructionScript`)